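; Linked portal actor that shows a live view through its partner and teleports the VR pawn when its camera crosses the plane.
; At startup it creates a viewport-sized render target for its material, fed by the linked portal's capture camera, and clips its own camera at the portal plane.
; Each tick, in post-update work, it mirrors the player camera to the partner and tests for crossings.
; Teleporting remaps transform, control rotation and velocity, then flags a camera cut.
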(event `self.ReceiveBeginPlay`
  (bind (_returnvalue_x _returnvalue_y) (`KismetMathLibrary.BreakVector2D` (`WidgetLayoutLibrary.GetViewportSize`)))
  (`KismetSystemLibrary.Delay` 0.1)
  (`self.SetTickGroup` "TG_PostUpdateWork")
  (bind _returnvalue (`KismetMaterialLibrary.CreateDynamicMaterialInstance` "/Game/Portals/Portal_MAT.Portal_MAT"))
  (bind _output_get (set `self.PortalMAT` _returnvalue))
  (`PrimitiveComponent.SetMaterial` (`self.PortalPllane`) 0 _output_get)
  (bind _returnvalue_2 (`KismetRenderingLibrary.CreateRenderTarget2D` (`KismetMathLibrary.FTrunc` _returnvalue_x) (`KismetMathLibrary.FTrunc` _returnvalue_y)))
  (bind _output_get_2 (set `self.PortalRT` _returnvalue_2))
  (`MaterialInstanceDynamic.SetTextureParameterValue` (`self.PortalMAT`) "Texture" _output_get_2)
  (set `SceneCaptureComponent2D.TextureTarget` (`self.PortalRT`) (`/Game/Portals/Portal_BP.PortalCamera` (`self.Linked Portal`)))
  (`self.SetClipPlanes`)
  (`MaterialInstanceDynamic.SetVectorParameterValue` (`self.PortalMAT`) "OffsetDistance" (`KismetMathLibrary.MakeColor` (.x (* (`SceneComponent.GetForwardVector` (`self.ForwardDirection`)) (`self.Offset Amount`))) (.y (* (`SceneComponent.GetForwardVector` (`self.ForwardDirection`)) (`self.Offset Amount`))) (.z (* (`SceneComponent.GetForwardVector` (`self.ForwardDirection`)) (`self.Offset Amount`)))))
  (set `self.hasstarted` true))

(event `self.ReceiveTick`
  (params (DeltaSeconds :type "Float (single-precision)"))
  (if (`self.hasstarted`)
    (`self.UpdateSceneCapture`)
    (`self.CheckViewportSize`)
    (`self.ShouldTeleport`)))

(fn `CheckViewportSize`
  (bind _portalrt (`self.PortalRT`))
  (bind (_x _y) (`KismetMathLibrary.BreakVector2D` (`WidgetLayoutLibrary.GetViewportSize`)))
  (bind (_x_2 _y_2) (`KismetMathLibrary.BreakVector2D` (`WidgetLayoutLibrary.GetViewportSize`)))
  (if (not (and (== _x (`TextureRenderTarget2D.SizeX` _portalrt)) (== _y (`TextureRenderTarget2D.SizeY` _portalrt))))
    (`KismetRenderingLibrary.ResizeRenderTarget2D` (`self.PortalRT`) (`KismetMathLibrary.FTrunc` _x_2) (`KismetMathLibrary.FTrunc` _y_2))))

(fn `IsPointCrossingPortal`
  (params (Point :type "Vector Structure") (PortalLocation :type "Vector Structure") (PortalNormal :type "Vector Structure"))
  (returns (Return :type Boolean))
  (locals (IsFront :type Boolean) (PortalPlane :type "Plane Structure") (IsInersect :type Boolean :default false) (IsCrossing :type Boolean :default false))
  (set `local.IsFront` (>= (`KismetMathLibrary.Dot_VectorVector` PortalNormal (- Point PortalLocation)) 0.0))
  (bind _output_get (set `local.PortalPlane` (`KismetMathLibrary.MakePlaneFromPointAndNormal` (`local.PortalLocation`) (`local.PortalNormal`))))
  (set `local.IsInersect` (`.ReturnValue` (`KismetMathLibrary.LinePlaneIntersection` (`self.Last Position`) (`local.Point`) _output_get)))
  (set `local.IsCrossing` (and (`local.IsInersect`) (not (`local.IsFront`)) (`self.LastInFront`)))
  (set `self.LastInFront` (`local.IsFront`))
  (set `self.Last Position` (`local.Point`))
  (return (`local.IsCrossing`)))

(fn `SetClipPlanes`
  (bind _portalcamera (`self.PortalCamera`))
  (`/Engine/EditorBlueprintResources/StandardMacros.IsValid` (`self.Linked Portal`)
    (:`Is Valid`
      (set `SceneCaptureComponent2D.bEnableClipPlane` true _portalcamera)
      (set `SceneCaptureComponent2D.ClipPlaneBase` (+ (`SceneComponent.K2_GetComponentLocation` (`self.PortalPllane`)) (* (`SceneComponent.GetForwardVector` (`self.ForwardDirection`)) -3.0)) _portalcamera)
      (set `SceneCaptureComponent2D.ClipPlaneNormal` (`SceneComponent.GetForwardVector` (`self.ForwardDirection`)) _portalcamera))))

(fn `ShouldTeleport`
  (`/Engine/EditorBlueprintResources/StandardMacros.IsValid` (`|GetArrayItem` (`PrimitiveComponent.GetOverlappingActors` (`self.PlayerDetection`) "/Game/VRTemplate/Blueprints/VRPawn.VRPawn_C"))
    (:`Is Valid`
      (bind _return (`self.IsPointCrossingPortal` (`SceneComponent.K2_GetComponentLocation` (`/Game/VRTemplate/Blueprints/VRPawn.Camera` (cast `/Game/VRTemplate/Blueprints/VRPawn` (`GameplayStatics.GetPlayerCharacter` 0) :!pure true))) (`self.K2_GetActorLocation`) (`SceneComponent.GetForwardVector` (`self.ForwardDirection`))))
      (if _return
        (`self.TeleportCharacter`)))))

(fn `TeleportCharacter`
  (bind _returnvalue (`self.GetTransform`))
  (bind _returnvalue_2 (`self.GetTransform`))
  (bind (_returnvalue_location _returnvalue_rotation _returnvalue_scale) (`KismetMathLibrary.BreakTransform` (`self.GetTransform`)))
  (bind _returnvalue_3 (`Pawn.GetMovementComponent` (`GameplayStatics.GetPlayerCharacter` 0)))
  (bind (_x _y _z) (`KismetMathLibrary.GetAxes` (`Controller.GetControlRotation` (`GameplayStatics.GetPlayerController` 0))))
  (bind (_x_2 _y_2 _z_2) (`KismetMathLibrary.GetAxes` (`self.K2_GetActorRotation` (`GameplayStatics.GetPlayerCharacter` 0))))
  (`self.K2_SetActorTransform` (`GameplayStatics.GetPlayerCharacter` 0) (`KismetMathLibrary.MakeTransform` (`KismetMathLibrary.TransformLocation` (`self.GetTransform` (`self.Linked Portal`)) (`KismetMathLibrary.InverseTransformLocation` (`KismetMathLibrary.MakeTransform` _returnvalue_location _returnvalue_rotation (`KismetMathLibrary.MakeVector` (* (.x _returnvalue_scale) -1.0) (* (.y _returnvalue_scale) -1.0) (.z _returnvalue_scale))) (`self.K2_GetActorLocation` (`GameplayStatics.GetPlayerCharacter` 0)))) (`KismetMathLibrary.MakeRotationFromAxes` (`KismetMathLibrary.TransformDirection` (`self.GetTransform` (`self.Linked Portal`)) (`KismetMathLibrary.MirrorVectorByNormal` (`KismetMathLibrary.MirrorVectorByNormal` (`KismetMathLibrary.InverseTransformDirection` _returnvalue_2 _x_2) (1.0 0.0 0.0)) (0.0 1.0 0.0))) (`KismetMathLibrary.TransformDirection` (`self.GetTransform` (`self.Linked Portal`)) (`KismetMathLibrary.MirrorVectorByNormal` (`KismetMathLibrary.MirrorVectorByNormal` (`KismetMathLibrary.InverseTransformDirection` _returnvalue_2 _y_2) (1.0 0.0 0.0)) (0.0 1.0 0.0))) (`KismetMathLibrary.TransformDirection` (`self.GetTransform` (`self.Linked Portal`)) (`KismetMathLibrary.MirrorVectorByNormal` (`KismetMathLibrary.MirrorVectorByNormal` (`KismetMathLibrary.InverseTransformDirection` _returnvalue_2 _z_2) (1.0 0.0 0.0)) (0.0 1.0 0.0))))) false false)
  (`Controller.SetControlRotation` (`GameplayStatics.GetPlayerController` 0) (`KismetMathLibrary.MakeRotationFromAxes` (`KismetMathLibrary.TransformDirection` (`self.GetTransform` (`self.Linked Portal`)) (`KismetMathLibrary.MirrorVectorByNormal` (`KismetMathLibrary.MirrorVectorByNormal` (`KismetMathLibrary.InverseTransformDirection` _returnvalue _x) (1.0 0.0 0.0)) (0.0 1.0 0.0))) (`KismetMathLibrary.TransformDirection` (`self.GetTransform` (`self.Linked Portal`)) (`KismetMathLibrary.MirrorVectorByNormal` (`KismetMathLibrary.MirrorVectorByNormal` (`KismetMathLibrary.InverseTransformDirection` _returnvalue _y) (1.0 0.0 0.0)) (0.0 1.0 0.0))) (`KismetMathLibrary.TransformDirection` (`self.GetTransform` (`self.Linked Portal`)) (`KismetMathLibrary.MirrorVectorByNormal` (`KismetMathLibrary.MirrorVectorByNormal` (`KismetMathLibrary.InverseTransformDirection` _returnvalue _z) (1.0 0.0 0.0)) (0.0 1.0 0.0)))))
  (bind _returnvalue_4 (`self.UpdateVelocity` (`MovementComponent.Velocity` _returnvalue_3)))
  (set `MovementComponent.Velocity` _returnvalue_4 _returnvalue_3)
  (`PlayerCameraManager.SetGameCameraCutThisFrame` (`GameplayStatics.GetPlayerCameraManager` 0)))

(fn `UpdateSceneCapture`
  (bind _returnvalue (`self.GetTransform`))
  (bind _returnvalue_2 (`self.GetTransform` (`self.Linked Portal`)))
  (bind (_x _y _z) (`KismetMathLibrary.BreakVector3f` (.scale (`self.GetTransform`))))
  (bind (_x_2 _y_2 _z_2) (`KismetMathLibrary.BreakRotIntoAxes` (`SceneComponent.K2_GetComponentRotation` (`PlayerCameraManager.TransformComponent` (`GameplayStatics.GetPlayerCameraManager` 0)))))
  (`SceneComponent.K2_SetWorldLocationAndRotation` (`/Game/Portals/Portal_BP.PortalCamera` (`self.Linked Portal`)) (`KismetMathLibrary.TransformLocation` (`self.GetTransform` (`self.Linked Portal`)) (`KismetMathLibrary.InverseTransformLocation` (`KismetMathLibrary.MakeTransform` (.location (`self.GetTransform`)) (.rotation (`self.GetTransform`)) (`KismetMathLibrary.MakeVector` (* _x -1.0) (* _y -1.0) _z)) (`SceneComponent.K2_GetComponentLocation` (`PlayerCameraManager.TransformComponent` (`GameplayStatics.GetPlayerCameraManager` 0))))) (`KismetMathLibrary.MakeRotationFromAxes` (`KismetMathLibrary.TransformDirection` _returnvalue_2 (`KismetMathLibrary.MirrorVectorByNormal` (`KismetMathLibrary.MirrorVectorByNormal` (`KismetMathLibrary.InverseTransformDirection` _returnvalue _x_2) (1.0 0.0 0.0)) (0.0 1.0 0.0))) (`KismetMathLibrary.TransformDirection` _returnvalue_2 (`KismetMathLibrary.MirrorVectorByNormal` (`KismetMathLibrary.MirrorVectorByNormal` (`KismetMathLibrary.InverseTransformDirection` _returnvalue _y_2) (1.0 0.0 0.0)) (0.0 1.0 0.0))) (`KismetMathLibrary.TransformDirection` _returnvalue_2 (`KismetMathLibrary.MirrorVectorByNormal` (`KismetMathLibrary.MirrorVectorByNormal` (`KismetMathLibrary.InverseTransformDirection` _returnvalue _z_2) (1.0 0.0 0.0)) (0.0 1.0 0.0)))) false false))

(fn `UpdateVelocity`
  (params (Velocity :type "Vector Structure"))
  (returns (ReturnValue :type "Vector Structure"))
  (return (* (`KismetMathLibrary.TransformDirection` (`self.GetTransform` (`self.Linked Portal`)) (`KismetMathLibrary.MirrorVectorByNormal` (`KismetMathLibrary.MirrorVectorByNormal` (`KismetMathLibrary.InverseTransformDirection` (`self.GetTransform`) (`KismetMathLibrary.Normal` Velocity)) (1.0 0.0 0.0)) (0.0 1.0 0.0))) (`KismetMathLibrary.VSize` (`local.Velocity`)))))

(fn `UserConstructionScript`)