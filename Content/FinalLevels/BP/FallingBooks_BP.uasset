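; FallingBooks_BP is a one-shot trigger that sends a book falling with a sound.
; The first overlap on the Box sets a flag, replaces the Book's linear velocity with the Movement vector and plays a 2D falling sound.
; After a short delay, physics simulation and collision are disabled on the Book, freezing it in place.
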(event `self.Box.OnComponentBeginOverlap`
  (params (OverlappedComponent :type "PrimitiveComponent Object Reference") (OtherActor :type "Actor Object Reference") (OtherComp :type "PrimitiveComponent Object Reference") (OtherBodyIndex :type Integer) (bFromSweep :type Boolean) (SweepResult :type "HitResult Structure (by ref)"))
  (bind _book (`self.book`))
  (if (not (`self.HasTriggerd`))
    (set `self.HasTriggerd` true)
    (`PrimitiveComponent.SetPhysicsLinearVelocity` (`self.book`) (`self.Movement`) false "None")
    (`GameplayStatics.PlaySound2D` "/Game/Sounds/BookFalling.BookFalling" 1.0 1.0 0.0 null null)
    (`KismetSystemLibrary.Delay` 3.0)
    (`PrimitiveComponent.SetSimulatePhysics` _book false)
    (`PrimitiveComponent.SetCollisionEnabled` _book "NoCollision")))

(fn `UserConstructionScript`)