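; Main menu Blueprint that provides two-handed pointer interaction with UI widgets through left and right widget interaction components.
; Every tick it destroys each side's spline mesh and, while that side is over a hit-testable widget, creates a new one from the component to the hit point as a pointer beam.
; Left and right shoot inputs press the left mouse button on the matching component, with no release call.
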(event `self.ReceiveTick`
  (params (DeltaSeconds :type "Float (single-precision)"))
  (`self.WidgetInteractionPointer`))

(event `EnhancedInput|/Game/VRTemplate/Input/Actions/IA_Shoot_Left`
  (params (ActionValue :type Boolean) (ElapsedSeconds :type "Float (double-precision)") (TriggeredSeconds :type "Float (double-precision)") (InputAction :type "InputAction Object Reference" :default "/Game/VRTemplate/Input/Actions/IA_Shoot_Left.IA_Shoot_Left"))
  (:`Triggered`
    (`WidgetInteractionComponent.PressPointerKey` (`self.WidgetInteractionLEFT`) "LeftMouseButton" :!label _label))
  (:`Started`
    (goto _label))
  (:`Ongoing`
    (goto _label)))

(event `EnhancedInput|/Game/VRTemplate/Input/Actions/IA_Shoot_Right`
  (params (ActionValue :type Boolean) (ElapsedSeconds :type "Float (double-precision)") (TriggeredSeconds :type "Float (double-precision)") (InputAction :type "InputAction Object Reference" :default "/Game/VRTemplate/Input/Actions/IA_Shoot_Right.IA_Shoot_Right"))
  (:`Triggered`
    (`WidgetInteractionComponent.PressPointerKey` (`self.WidgetInteractionRIGHT`) "LeftMouseButton" :!label _label_2))
  (:`Started`
    (goto _label_2))
  (:`Ongoing`
    (goto _label_2)))

(fn `UserConstructionScript`)

(fn `WidgetInteractionPointer`
  (bind _widgetinteractionleft (`self.WidgetInteractionLEFT`))
  (bind _widgetinteractionright (`self.WidgetInteractionRIGHT`))
  (bind (_returnvalue_bblockinghit _returnvalue_binitialoverlap _returnvalue_time _returnvalue_distance _returnvalue_location) (`GameplayStatics.BreakHitResult` (`WidgetInteractionComponent.GetLastHitResult` _widgetinteractionleft)))
  (bind _returnvalue (`SceneComponent.K2_GetComponentLocation` _widgetinteractionleft))
  (bind _returnvalue_2 (`SceneComponent.K2_GetComponentLocation` _widgetinteractionright))
  (bind (_returnvalue_bblockinghit_2 _returnvalue_binitialoverlap_2 _returnvalue_time_2 _returnvalue_distance_2 _returnvalue_location_2) (`GameplayStatics.BreakHitResult` (`WidgetInteractionComponent.GetLastHitResult` _widgetinteractionright)))
  (bind _returnvalue_3 (`KismetMathLibrary.GetForwardVector` (`KismetMathLibrary.FindLookAtRotation` _returnvalue _returnvalue_location)))
  (bind _returnvalue_4 (`KismetMathLibrary.GetForwardVector` (`KismetMathLibrary.FindLookAtRotation` _returnvalue_2 _returnvalue_location_2)))
  (`|ExecutionSequence`
    (:`then_0`
      (bind _leftsplinemesh (`self.LeftSplineMesh`)
        (:`then`
          (`ActorComponent.K2_DestroyComponent` _leftsplinemesh))
        (:`else`
          _))
      (if (`WidgetInteractionComponent.IsOverHitTestVisibleWidget` _widgetinteractionleft)
        (bind _returnvalue_5 (`AddComponent|NODE_AddSplineMeshComponent-0`))
        (bind _output_get (set `self.LeftSplineMesh` _returnvalue_5))
        (`SplineMeshComponent.SetStartAndEnd` (`self.LeftSplineMesh`) _returnvalue _returnvalue_3 _returnvalue_location (* _returnvalue_3 (`KismetMathLibrary.Conv_DoubleToVector` -1.0)) true)
        (`SplineMeshComponent.SetStartAndEnd` _output_get _returnvalue _returnvalue_3 _returnvalue_location (* _returnvalue_3 (`KismetMathLibrary.Conv_DoubleToVector` -1.0)) true)))
    (:`then_1`
      (bind _rightsplinemesh (`self.RightSplineMesh`)
        (:`then`
          (`ActorComponent.K2_DestroyComponent` _rightsplinemesh))
        (:`else`
          _))
      (if (`WidgetInteractionComponent.IsOverHitTestVisibleWidget` _widgetinteractionright)
        (bind _returnvalue_6 (`AddComponent|NODE_AddSplineMeshComponent-1`))
        (bind _output_get_2 (set `self.RightSplineMesh` _returnvalue_6))
        (`SplineMeshComponent.SetStartAndEnd` _output_get_2 _returnvalue_2 _returnvalue_4 _returnvalue_location_2 (* _returnvalue_4 (`KismetMathLibrary.Conv_DoubleToVector` -1.0)) true)))))